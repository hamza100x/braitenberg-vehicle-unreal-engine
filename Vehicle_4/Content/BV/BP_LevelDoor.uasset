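; BP_LevelDoor is a level-select door that shows its level number and loads that level when the player enters it.
; Overlaps starting or ending on DoorRadius toggle a FlipFlop that plays or reverses a timeline swinging the door 90 degrees, with no actor filter.
; TriggerBox reacts only to BP_ThirdPersonCharacter, swaps all widgets for a UW_CarBVLevel loading animation, then opens the mapped level after a delay.
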(event OnComponentBeginOverlap(TriggerBox)
  (params (OverlappedComponent :type Primitive%20Component%20Object%20Reference) (OtherActor :type Actor%20Object%20Reference) (OtherComp :type Primitive%20Component%20Object%20Reference) (OtherBodyIndex :type Integer) (bFromSweep :type Boolean) (SweepResult :type Hit%20Result%20Structure%20%28by%20ref%29))
  (Utilities|Casting|CastToBP_ThirdPersonCharacter OtherActor)
  (Audio|PlaySound2D "/Game/Audio/UI/level_up_2.level_up_2" 1.0 1.0 0.0 0 0)
  (Viewport|RemoveAllWidgets)
  (bind _returnvalue (UserInterface|CreateWidget "/Game/BV/UW_CarBVLevel.UW_CarBVLevel_C" (Game|GetPlayerController 0)))
  (UserInterface|Viewport|AddtoViewport _returnvalue 0)
  (Default|LoadingAnim _returnvalue)
  (Utilities|FlowControl|Delay 2.0)
  (Game|OpenLevel(byName) (.Value (Utilities|Map|Find (Variables|Default|GetLevelmap) (Variables|Default|GetLevel)))))

(event OnComponentBeginOverlap(DoorRadius)
  (params (OverlappedComponent :type Primitive%20Component%20Object%20Reference) (OtherActor :type Actor%20Object%20Reference) (OtherComp :type Primitive%20Component%20Object%20Reference) (OtherBodyIndex :type Integer) (bFromSweep :type Boolean) (SweepResult :type Hit%20Result%20Structure%20%28by%20ref%29))
  (CallFunction|OpenDoor))

(event OnComponentEndOverlap(DoorRadius)
  (params (OverlappedComponent :type Primitive%20Component%20Object%20Reference) (OtherActor :type Actor%20Object%20Reference) (OtherComp :type Primitive%20Component%20Object%20Reference) (OtherBodyIndex :type Integer))
  (CallFunction|OpenDoor))

(event Custom|OpenDoor
  (Utilities|FlowControl|FlipFlop
    (:A
      (bind _doorload (Timeline|OpenDoorTimeLine PlayFromStart)
        (:Update
          (Transformation|SetRelativeRotation (Variables|Default|GetDoor) (Math|Rotator|MakeRotator 0.0 0.0 (Math|Float|Lerp 0.0 9e+01 _doorload)) false false))))
    (:B
      (Timeline|OpenDoorTimeLine Reverse))))

(event EventBeginPlay
  (Rendering|Components|TextRender|SetText (Variables|Default|GetLevelText) (Utilities|Text|FormatText "Level {lvl}" (Variables|Default|GetLevel))))

(fn ConstructionScript)