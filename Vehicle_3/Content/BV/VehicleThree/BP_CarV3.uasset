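; BP_CarV3 is a self-driving, Braitenberg-style vehicle that reacts to nearby actors with "source" in their display name.
; Each Tick, a debug-drawn sphere trace finds sources and updates steering, throttle and an optional info widget.
; Crossed excitatory and inhibitory sensor components turn source distance into left and right values, averaged into one throttle.
; Steering comes separately from the scaled world-space look-at yaw toward the source, ignoring car heading.
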(event Custom|ScrubTrace
  (bind _returnvalue (Transformation|GetActorLocation))
  (bind _outhits (Collision|MultiSphereTraceForObjects _returnvalue _returnvalue 2.8e+03 (Variables|Default|GetObject%20Types) false 0 "ForDuration" true "(R=0.088195,G=1.000000,B=0.100112,A=1.000000)" "(R=0.096851,G=1.000000,B=0.053332,A=1.000000)" 1.0))
  (for _array_element _outhits
    (if (Utilities|String|Contains (Utilities|GetDisplayName (.HitActor (Collision|BreakHitResult _array_element))) "source")
      (Variables|Default|SethitLocation (Transformation|GetActorLocation (.HitActor (Collision|BreakHitResult _array_element))))
      (bind (_left _right) (CallFunction|GetthrottleInputs))
      (bind _steering (CallFunction|GetSteeringAngle))
      (bind _output_get (Variables|Default|SetAngle _steering))
      (Class|ChaosVehicleMovementComponent|SetSteeringInput (Variables|Default|GetVehicleMovementComponent) _output_get)
      (bind _output_get_2 (Variables|Default|SetThrottle (* (Math|Float|Absolute(Float) (/ (+ _left _right) 2.0)) 0.6)))
      (Class|ChaosVehicleMovementComponent|SetThrottleInput (Variables|Default|GetVehicleMovementComponent) _output_get_2)
      ;[1 1 1] WidgetUpdate
      (if (Variables|Default|Getinfo?)
        (if (Variables|Default|GetinfoUp)
          _
          (else
            (bind _returnvalue_2 (UserInterface|CreateWidget "/Game/BV/UI/UW_CarInfo.UW_CarInfo_C" (Game|GetPlayerController 0)))
            (bind _output_get_3 (Variables|Default|SetcarinfoWidget _returnvalue_2))
            (UserInterface|Viewport|AddtoViewport _output_get_3 0)
            (Variables|Default|SetinfoUp true)))
        (Variables|/Script/UMG.TextBlock|SetText (Variables|/Game/BV/UI/UW_CarInfo.UW_CarInfo_C|GetThrottle (Variables|Default|GetcarinfoWidget)) (Utilities|Text|ToText(Float) (Variables|Default|GetThrottle) "HalfToEven"))
        (Variables|/Script/UMG.TextBlock|SetText (Variables|/Game/BV/UI/UW_CarInfo.UW_CarInfo_C|GetAngle (Variables|Default|GetcarinfoWidget)) (Utilities|Text|ToText(Float) (Variables|Default|GetAngle) "HalfToEven"))
        (Variables|/Script/UMG.TextBlock|SetText (Variables|/Game/BV/UI/UW_CarInfo.UW_CarInfo_C|GetNMR (Variables|Default|GetcarinfoWidget)) (Utilities|Text|ToText(Integer) (Variables|Default|GetNMR)))
        (Variables|/Script/UMG.TextBlock|SetText (Variables|/Game/BV/UI/UW_CarInfo.UW_CarInfo_C|GetWeight (Variables|Default|GetcarinfoWidget)) (Utilities|Text|ToText(Float) (Variables|Default|GetWeight) "HalfToEven"))
        (Variables|/Script/UMG.TextBlock|SetText (Variables|/Game/BV/UI/UW_CarInfo.UW_CarInfo_C|GetVehicleName (Variables|Default|GetcarinfoWidget)) (Utilities|Text|ToText(Name) (Variables|Default|GetCarname)))
        (else
          (bind _carinfowidget (Variables|Default|GetcarinfoWidget)
            (:then
              (Widget|RemovefromParent _carinfowidget)
              (Variables|Default|SetinfoUp false))
            (:else)))))))

(event EventTick
  (params (DeltaSeconds :type Float%20%28single-precision%29))
  (Variables|Default|Setcar%20location (Transformation|GetActorLocation))
  (CallFunction|ScrubTrace))

(fn ConstructionScript)

(fn GetSensorinput
  (params (Sensor :type Vector))
  (return (Math|Float|Absolute(Float) (Math|Float|NormalizetoRange (/ (Math|Vector|VectorLength (- (Variables|Default|GethitLocation) Sensor)) 3e+01) 0.0 1.0))))

(fn GetthrottleInputs
  ;[1 1 1] Left Throttle Input
  (bind _sensorout (CallFunction|GetSensorinput (Transformation|GetWorldLocation (Variables|Default|GetExciRight1))))
  (bind _sensorout_2 (CallFunction|GetSensorinput (Transformation|GetWorldLocation (Variables|Default|GetExciRight2))))
  (bind _sensorout_3 (CallFunction|GetSensorinput (Transformation|GetWorldLocation (Variables|Default|GetExciRight3))))
  (bind _sensorout_4 (CallFunction|GetSensorinput (Transformation|GetWorldLocation (Variables|Default|GetExciRight4))))
  (bind _sensorout_5 (CallFunction|GetSensorinput (Transformation|GetWorldLocation (Variables|Default|GetExciRight5))))
  (bind _sensorout_6 (CallFunction|GetSensorinput (Transformation|GetWorldLocation (Variables|Default|GetInhiRight3))))
  (bind _sensorout_7 (CallFunction|GetSensorinput (Transformation|GetWorldLocation (Variables|Default|GetInhiRight2))))
  (bind _sensorout_8 (CallFunction|GetSensorinput (Transformation|GetWorldLocation (Variables|Default|GetInhiRight1))))
  ;[1 1 1] Right Throttle Input
  (bind _sensorout_9 (CallFunction|GetSensorinput (Transformation|GetWorldLocation (Variables|Default|GetExciLeft1))))
  (bind _sensorout_10 (CallFunction|GetSensorinput (Transformation|GetWorldLocation (Variables|Default|GetExciLeft2))))
  (bind _sensorout_11 (CallFunction|GetSensorinput (Transformation|GetWorldLocation (Variables|Default|GetExciLeft3))))
  (bind _sensorout_12 (CallFunction|GetSensorinput (Transformation|GetWorldLocation (Variables|Default|GetExciLeft4))))
  (bind _sensorout_13 (CallFunction|GetSensorinput (Transformation|GetWorldLocation (Variables|Default|GetExciLeft5))))
  (bind _sensorout_14 (CallFunction|GetSensorinput (Transformation|GetWorldLocation (Variables|Default|GetInhiLeft3))))
  (bind _sensorout_15 (CallFunction|GetSensorinput (Transformation|GetWorldLocation (Variables|Default|GetInhiLeft2))))
  (bind _sensorout_16 (CallFunction|GetSensorinput (Transformation|GetWorldLocation (Variables|Default|GetInhiLeft1))))
  (return (- (/ (+ _sensorout _sensorout_2 _sensorout_3 _sensorout_4 _sensorout_5) 5.0) (/ (+ _sensorout_8 _sensorout_7 _sensorout_6) 3.0)) (- (/ (+ _sensorout_9 _sensorout_10 _sensorout_11 _sensorout_12 _sensorout_13) 5.0) (/ (+ _sensorout_16 _sensorout_15 _sensorout_14) 3.0))))

(fn GetSteeringAngle
  (return (* (/ (.yaw (Math|Rotator|FindLookatRotation (Variables|Default|Getcar%20location) (Variables|Default|GethitLocation))) 3.6e+02) 1.3)))