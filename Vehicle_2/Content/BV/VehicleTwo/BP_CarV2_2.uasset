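; Sensor-driven car Blueprint that steers and throttles in response to a source location passed into MoveForward.
; Steering comes from the world-space look-at yaw from car to source, scaled by a smoother.
; Throttle combines left and right sensor proximity, averaged by sensor count and damped, so it rises nearer the source.
; An optional on-screen widget shows throttle, angle and vehicle details while Info is enabled.
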(event Custom|MoveForward
  (params (sourceLocation :type Vector))
  (bind _nmrsensors (Variables|Default|GetnmrSensors))
  (bind _throttleleft (Variables|Default|GetthrottleLeft))
  (bind _vehiclemovementcomponent (Variables|Default|GetVehicleMovementComponent))
  (bind _throttleright (Variables|Default|Getthrottleright))
  (bind _returnvalue (+ _throttleright _throttleleft))
  (bind _returnvalue_2 (/ _returnvalue _nmrsensors))
  (bind _returnvalue_3 (* _returnvalue_2 0.6))
  ;[0 0 0] Move Forward
  (Variables|Default|SetSourcelocation sourceLocation)
  (bind _steeringangle (CallFunction|GetSteeringAngle))
  (CallFunction|GetThrottleInputs)
  (bind _output_get (Variables|Default|SetAngle _steeringangle))
  (Class|ChaosVehicleMovementComponent|SetSteeringInput _vehiclemovementcomponent _output_get)
  (Class|ChaosVehicleMovementComponent|SetThrottleInput _vehiclemovementcomponent _returnvalue_3)
  (Variables|Default|SetThrottle _returnvalue_3)
  ;[1 1 1] WidgetUpdate
  (if (Variables|Default|Getinfo?)
    (if (Variables|Default|GetinfoUp)
      _
      (else
        (bind _returnvalue_4 (UserInterface|CreateWidget "/Game/BV/UI/UW_CarInfo.UW_CarInfo_C" (Game|GetPlayerController 0)))
        (bind _output_get_2 (Variables|Default|SetcarinfoWidget _returnvalue_4))
        (UserInterface|Viewport|AddtoViewport _output_get_2 0)
        (Variables|Default|SetinfoUp true)))
    (Variables|/Script/UMG.TextBlock|SetText (Variables|/Game/BV/UI/UW_CarInfo.UW_CarInfo_C|GetThrottle (Variables|Default|GetcarinfoWidget)) (Utilities|Text|ToText(Float) (Variables|Default|GetThrottle) "HalfToEven"))
    (Variables|/Script/UMG.TextBlock|SetText (Variables|/Game/BV/UI/UW_CarInfo.UW_CarInfo_C|GetAngle (Variables|Default|GetcarinfoWidget)) (Utilities|Text|ToText(Float) (Variables|Default|GetAngle) "HalfToEven"))
    (Variables|/Script/UMG.TextBlock|SetText (Variables|/Game/BV/UI/UW_CarInfo.UW_CarInfo_C|GetNMR (Variables|Default|GetcarinfoWidget)) (Utilities|Text|ToText(Integer) (Variables|Default|GetNMR)))
    (Variables|/Script/UMG.TextBlock|SetText (Variables|/Game/BV/UI/UW_CarInfo.UW_CarInfo_C|GetWeight (Variables|Default|GetcarinfoWidget)) (Utilities|Text|ToText(Float) (Variables|Default|GetWeight) "HalfToEven"))
    (Variables|/Script/UMG.TextBlock|SetText (Variables|/Game/BV/UI/UW_CarInfo.UW_CarInfo_C|GetVehicleName (Variables|Default|GetcarinfoWidget)) (Utilities|Text|ToText(Name) (Variables|Default|GetCarname)))
    (else
      (bind _carinfowidget (Variables|Default|GetcarinfoWidget)
        (:then
          (Widget|RemovefromParent _carinfowidget)
          (Variables|Default|SetinfoUp false))
        (:else)))))

(fn ConstructionScript)

(fn GetSensorLocation
  (return (Transformation|GetWorldLocation (Variables|Default|GetSensorLeft)) (Transformation|GetWorldLocation (Variables|Default|GetSensorRight))))

(fn GetThrottleInputs
  (bind (_sesonlocationleft _sesonlocationright) (CallFunction|GetSensorLocation))
  (Variables|Default|SetthrottleLeft (- 1.0 (Math|Float|NormalizetoRange (Math|Float|NormalizetoRange (/ (Math|Vector|VectorLength (- (Variables|Default|GetSourcelocation) _sesonlocationleft)) 5e+03) 0.0 1.0) 0.0 1.0)))
  (Variables|Default|Setthrottleright (- 1.0 (Math|Float|NormalizetoRange (Math|Float|NormalizetoRange (/ (Math|Vector|VectorLength (- (Variables|Default|GetSourcelocation) _sesonlocationright)) 5e+03) 0.0 1.0) 0.0 1.0))))

(fn GetSteeringAngle
  (return (* (/ (.yaw (Math|Rotator|FindLookatRotation (Transformation|GetActorLocation) (Variables|Default|GetSourcelocation))) 3.6e+02) (Variables|Default|GetSteeringSmoother))))